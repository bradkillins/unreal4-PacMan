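; Player controller for the Pacman game that toggles the pause menu.
; The Pause input and PauseEvent share one branch that checks whether a stored pause widget is still valid.
; If none exists, it creates UMG_PauseMenu, pauses the game, shows the cursor and hides the Pacman HUD.
; Otherwise it removes the widget, unpauses, restores game-only input and turns the HUD back on.
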(event Custom|PauseEvent
  (bind _returnvalue (Game|GetPlayerController 0))
  (bind _returnvalue_2 (Game|GetPlayerCharacter 0))
  (bind _returnvalue_3 (Game|GetPlayerController 0))
  (bind _aspacman (Utilities|Casting|CastToPacman _returnvalue_2))
  ;[1 1 1] Check if Pause Screen is already displayed
  (Utilities|IsValid (Variables|Default|GetPauseUIReference)
    (:Is%20Valid
      ;[1 1 1] Destroy Pause Menu, Unpause game, Toggle HUD
      (Widget|RemovefromParent (Variables|Default|GetPauseUIReference))
      (Variables|Default|SetPauseUIReference 0)
      (Input|SetInputModeGameOnly _returnvalue)
      (Variables|/Script/Engine.PlayerController|SetbShowMouseCursor _returnvalue false)
      (Game|SetGamePaused false)
      (Default|HudON _aspacman))
    (:Is%20Not%20Valid
      ;[1 1 1] Create Pause Menu, Pause Game and Toggle HUD
      (bind _returnvalue_4 (UserInterface|CreateWidget "/Game/UI/UMG_PauseMenu.UMG_PauseMenu_C"))
      (bind _output_get (Variables|Default|SetPauseUIReference _returnvalue_4))
      (UserInterface|Viewport|AddtoViewport _output_get 0)
      (Input|SetInputModeGameandUI _returnvalue_3 0 "DoNotLock" true)
      (Variables|/Script/Engine.PlayerController|SetbShowMouseCursor _returnvalue_3 true)
      (Game|SetGamePaused true)
      (Default|HudOFF _aspacman))))

(event Input|ActionEvents|InputActionPause
  (params (Key :type Key%20Structure :default "None"))
  (bind _returnvalue (Game|GetPlayerController 0))
  (bind _returnvalue_2 (Game|GetPlayerCharacter 0))
  (bind _returnvalue_3 (Game|GetPlayerController 0))
  (bind _aspacman (Utilities|Casting|CastToPacman _returnvalue_2))
  (:Pressed
    ;[1 1 1] Check if Pause Screen is already displayed
    (Utilities|IsValid (Variables|Default|GetPauseUIReference)
      (:Is%20Valid
        ;[1 1 1] Destroy Pause Menu, Unpause game, Toggle HUD
        (Widget|RemovefromParent (Variables|Default|GetPauseUIReference))
        (Variables|Default|SetPauseUIReference 0)
        (Input|SetInputModeGameOnly _returnvalue)
        (Variables|/Script/Engine.PlayerController|SetbShowMouseCursor _returnvalue false)
        (Game|SetGamePaused false)
        (Default|HudON _aspacman))
      (:Is%20Not%20Valid
        ;[1 1 1] Create Pause Menu, Pause Game and Toggle HUD
        (bind _returnvalue_4 (UserInterface|CreateWidget "/Game/UI/UMG_PauseMenu.UMG_PauseMenu_C"))
        (bind _output_get (Variables|Default|SetPauseUIReference _returnvalue_4))
        (UserInterface|Viewport|AddtoViewport _output_get 0)
        (Input|SetInputModeGameandUI _returnvalue_3 0 "DoNotLock" true)
        (Variables|/Script/Engine.PlayerController|SetbShowMouseCursor _returnvalue_3 true)
        (Game|SetGamePaused true)
        (Default|HudOFF _aspacman)))))

(fn ConstructionScript)